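; BP_Ball is a player-controlled physics ball that rolls, jumps and keeps a score.
; MoveForward and MoveRight axis inputs roll BallMesh by applying world-axis torque as acceleration, independent of mass.
; Jump applies an upward velocity-change impulse, gated by IsJumping until any Hit event clears it, including wall contacts.
; IncrementScore adds a given amount to Score, with no caller in this Blueprint.
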(event `InputAxis|MoveForward`
  (params (AxisValue :type "Float (single-precision)"))
  ;[1 1 1] Moving
  (`PrimitiveComponent.AddTorqueInDegrees` (`self.BallMesh`) (`KismetMathLibrary.MakeVector` 0.0 (* AxisValue 1000.0)) "None" true))

(event `InputAction|Jump`
  (params (Key :type "Key Structure"))
  ;[1 1 1] Jumping
  (:`Pressed`
    (if (not (`self.isJumping`))
      (`PrimitiveComponent.AddImpulse` (`self.BallMesh`) (`KismetMathLibrary.MakeVector` 0.0 0.0 600.0) "None" true)
      (set `self.isJumping` true))))

(event `self.ReceiveHit`
  (params (MyComp :type "PrimitiveComponent Object Reference") (Other :type "Actor Object Reference") (OtherComp :type "PrimitiveComponent Object Reference") (bSelfMoved :type Boolean) (HitLocation :type "Vector Structure") (HitNormal :type "Vector Structure") (NormalImpulse :type "Vector Structure") (Hit :type "HitResult Structure (by ref)"))
  ;[1 1 1] Jumping
  (set `self.isJumping` false))

(event `InputAxis|MoveRight`
  (params (AxisValue :type "Float (single-precision)"))
  ;[1 1 1] Moving
  (`PrimitiveComponent.AddTorqueInDegrees` (`self.BallMesh`) (`KismetMathLibrary.MakeVector` (* AxisValue -1000.0)) "None" true))

(fn `IncrementScore`
  (params (InScore :type Integer))
  (set `self.Score` (+ InScore (`self.Score`))))

(fn `UserConstructionScript`)